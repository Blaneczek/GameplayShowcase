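; Sprint gameplay ability that raises the avatar's movement speed while input is held.
; On activation it applies the GE_Sprint effect to the owner and sets a faster speed through a movement speed message to the avatar.
; It ends on input release or on a movement-stopped gameplay event from the avatar.
; Ending removes the stored effect handle and restores the default speed.
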(event `self.K2_ActivateAbility`
  (bind _returnvalue (`AbilitySystemBlueprintLibrary.MakeSpecHandleByClass` "/Game/Blueprints/AbilitySystem/Effects/Abilities/Sprint/GE_Sprint.GE_Sprint_C"))
  (bind _returnvalue_2 (`self.K2_ApplyGameplayEffectSpecToOwner` _returnvalue))
  (message `GSAbilityCharacterHelper.SetMovementSpeed` (`self.GetAvatarActorFromActorInfo`) 1000.0 false)
  (`AbilityTask_WaitInputRelease.WaitInputRelease` true
    (:`then`
      (`AbilityAsync_WaitGameplayEvent.WaitGameplayEventToActor` (`self.GetAvatarActorFromActorInfo`) (struct :`TagName` "Event.Character.Movement.Stopped")
        (:`EventReceived`
          _)))
    (:`OnRelease`
      _))
  (`self.K2_EndAbility`))

(event `self.K2_OnEndAbility`
  (params (bWasCancelled :type Boolean))
  (`self.BP_RemoveGameplayEffectFromOwnerWithHandle` (stale `self.K2_ActivateAbility` _returnvalue_2))
  (message `GSAbilityCharacterHelper.SetMovementSpeed` (`self.GetAvatarActorFromActorInfo`) 0.0 true))