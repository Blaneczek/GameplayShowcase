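; BP_ItemSpawnerDEBUG is a debug actor that spawns items through GSLoot.
; Its Sphere overlap registers the spawner on a BP_PlayerWarrior when the player enters and clears that reference on exit.
; SpawnItems calls GSLoot's SpawnItems and prints a test string; nothing in this Blueprint calls it.
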(event `self.Sphere.OnComponentBeginOverlap`
  (params (OverlappedComponent :type "PrimitiveComponent Object Reference") (OtherActor :type "Actor Object Reference") (OtherComp :type "PrimitiveComponent Object Reference") (OtherBodyIndex :type Integer) (bFromSweep :type Boolean) (SweepResult :type "HitResult Structure (by ref)"))
  (bind _asbp_player_warrior (cast `/Game/Blueprints/Characters/Player/BP_PlayerWarrior` OtherActor))
  (`/Engine/EditorBlueprintResources/StandardMacros.IsValid` _asbp_player_warrior
    (:`Is Valid`
      (set `/Game/Blueprints/Characters/Player/BP_PlayerWarrior.ItemSpawnerDEBUG` self _asbp_player_warrior))))

(event `self.Sphere.OnComponentEndOverlap`
  (params (OverlappedComponent :type "PrimitiveComponent Object Reference") (OtherActor :type "Actor Object Reference") (OtherComp :type "PrimitiveComponent Object Reference") (OtherBodyIndex :type Integer))
  (bind _asbp_player_warrior (cast `/Game/Blueprints/Characters/Player/BP_PlayerWarrior` OtherActor))
  (`/Engine/EditorBlueprintResources/StandardMacros.IsValid` _asbp_player_warrior
    (:`Is Valid`
      (set `/Game/Blueprints/Characters/Player/BP_PlayerWarrior.ItemSpawnerDEBUG` null _asbp_player_warrior))))

(fn `SpawnItems`
  (`GSLootComponent.SpawnItems` (`self.GSLoot`))
  (`KismetSystemLibrary.PrintString` "Hello"))

(fn `UserConstructionScript`)