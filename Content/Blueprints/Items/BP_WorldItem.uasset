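; BP_WorldItem is a world item Blueprint that shows the item's name through a NameWidget.
; When the ItemNameSet event fires, it appends "+" and the upgrade level to the name if the level is below 90, otherwise keeping the plain name.
; It then casts the widget's user object to WBP_ItemDisplayName and passes it the text.
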(event `self.ItemNameSet`
  (params (Name :type "Text (by ref)") (UpgradeLevel :type Integer))
  (if (< UpgradeLevel 90)
    (set `self.Name` (`|FormatText` "{0}+{1}" Name UpgradeLevel))
    (else
      (set `self.Name` Name)))
  (bind _aswbp_item_display_name (cast `/Game/Blueprints/UI/Gameplay/Utility/WBP_ItemDisplayName` (`WidgetComponent.GetUserWidgetObject` (`self.NameWidget`))))
  (`/Engine/EditorBlueprintResources/StandardMacros.IsValid` _aswbp_item_display_name
    (:`Is Valid`
      (`/Game/Blueprints/UI/Gameplay/Utility/WBP_ItemDisplayName.SetItemName` _aswbp_item_display_name (`self.Name`)))))

(fn `UserConstructionScript`)